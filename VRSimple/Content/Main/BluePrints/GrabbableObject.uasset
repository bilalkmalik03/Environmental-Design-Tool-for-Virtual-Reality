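; Grabbable actor that floats without gravity and can be resized per axis.
; Gravity is off from construction; when GrabComponent reports a drop, it is disabled again and linear and angular velocity are zeroed so the mesh stops in place.
; ScaleX, ScaleY and ScaleZ each set one axis of the mesh's relative scale to a clamped 0–1 input times the MaxScale–MinScale range, without adding MinScale as an offset.
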(event `self.GrabComponent.OnDropped`
  (bind _staticmesh (`self.StaticMesh`))
  (`PrimitiveComponent.SetEnableGravity` _staticmesh false)
  (`PrimitiveComponent.SetPhysicsLinearVelocity` _staticmesh (0.0 0.0 0.0) false "None")
  (`PrimitiveComponent.SetPhysicsAngularVelocityInDegrees` _staticmesh (0.0 0.0 0.0) false "None"))

(fn `ScaleX`
  (params (scale :type "Float (double-precision)"))
  (bind _staticmesh (`self.StaticMesh`))
  (bind (_relativescale3d_x _relativescale3d_y _relativescale3d_z) (`KismetMathLibrary.BreakVector` (`SceneComponent.RelativeScale3D` _staticmesh)))
  (`SceneComponent.SetRelativeScale3D` _staticmesh (`KismetMathLibrary.MakeVector` (* (- (`self.maxScale`) (`self.minScale`)) (`KismetMathLibrary.FClamp` scale)) _relativescale3d_y _relativescale3d_z)))

(fn `ScaleY`
  (params (scale :type "Float (double-precision)"))
  (bind _staticmesh (`self.StaticMesh`))
  (bind (_relativescale3d_x _relativescale3d_y _relativescale3d_z) (`KismetMathLibrary.BreakVector` (`SceneComponent.RelativeScale3D` _staticmesh)))
  (`SceneComponent.SetRelativeScale3D` _staticmesh (`KismetMathLibrary.MakeVector` _relativescale3d_x (* (- (`self.maxScale`) (`self.minScale`)) (`KismetMathLibrary.FClamp` scale)) _relativescale3d_z)))

(fn `ScaleZ`
  (params (scale :type "Float (double-precision)"))
  (bind _staticmesh (`self.StaticMesh`))
  (bind (_relativescale3d_x _relativescale3d_y) (`KismetMathLibrary.BreakVector` (`SceneComponent.RelativeScale3D` _staticmesh)))
  (`SceneComponent.SetRelativeScale3D` _staticmesh (`KismetMathLibrary.MakeVector` _relativescale3d_x _relativescale3d_y (* (- (`self.maxScale`) (`self.minScale`)) (`KismetMathLibrary.FClamp` scale)))))

(fn `UserConstructionScript`
  (`PrimitiveComponent.SetEnableGravity` (`self.StaticMesh`) false))